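; Enemy character that attacks survivors, installs traps and exposes walk-speed control.
; Attack enables a collision that AttackEnd switches off; overlapping a survivor damages it, passing whether both face the same way via a forward-vector dot product.
; It also binds the survivor's damage-to-enemy event, which changes the enemy's state and ends the attack.
; State lives in ABP_Enemy, set by these actions and read through GetState.
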(event OnComponentBeginOverlap(AttackCollision)
  (params (OverlappedComponent :type Primitive%20Component%20Object%20Reference) (OtherActor :type Actor%20Object%20Reference) (OtherComp :type Primitive%20Component%20Object%20Reference) (OtherBodyIndex :type Integer) (bFromSweep :type Boolean) (SweepResult :type Hit%20Result%20Structure%20%28by%20ref%29))
  (bind _asbp_character_survivor (Utilities|Casting|CastToBP_Character_Survivor OtherActor))
  (EventDispatchers|BindEventtoOnDamagetoEnemy _asbp_character_survivor (delegate Custom|Event%20Damage%20By%20Survivor))
  (Class|UnderWorldCharacter|Damage _asbp_character_survivor (>= (Math|Vector|DotProduct (Transformation|GetActorForwardVector _asbp_character_survivor) (Transformation|GetActorForwardVector self)) 0.0)))

(event Custom|Event%20Attack%20End
  (Variables|/Script/Engine.PrimitiveComponent|SetbGenerateOverlapEvents (Variables|Default|GetAttackCollision) false))

(event Custom|Event%20Damage%20By%20Survivor
  (bind _asabp_enemy (Utilities|Casting|CastToABP_Enemy (Components|SkeletalMesh|GetAnimInstance (Variables|Character|GetMesh))))
  (Variables|/Game/AI/Enemy/Animations/ABP_Enemy.ABP_Enemy_C|SetState _asabp_enemy "NewEnumerator4")
  (Utilities|Casting|CastToBP_EnemyController (Pawn|GetController self))
  (CallFunction|EventAttackEnd))

(event EventBeginPlay
  (CallFunction|EventAttackEnd))

(fn ConstructionScript)

(fn UpdateWalkSpeed
  (params (NewWalkSpeed :type Float%20%28double-precision%29))
  (Variables|/Script/Engine.CharacterMovementComponent|SetMaxWalkSpeed (Variables|Character|GetCharacterMovement) NewWalkSpeed))

(fn InstallTrap
  (Game|SpawnActorfromClass "/Game/Blueprints/BP_Trap.BP_Trap_C" (Transformation|GetWorldTransform (Variables|Default|GetTrapSpawn)) "Undefined" "MultiplyWithRoot" 0 0)
  (bind _asabp_enemy (Utilities|Casting|CastToABP_Enemy (Components|SkeletalMesh|GetAnimInstance (Variables|Character|GetMesh))))
  (Variables|/Game/AI/Enemy/Animations/ABP_Enemy.ABP_Enemy_C|SetState _asabp_enemy "NewEnumerator2"))

(fn Attack
  (Variables|/Script/Engine.PrimitiveComponent|SetbGenerateOverlapEvents (Variables|Default|GetAttackCollision) true)
  (bind _asabp_enemy (Utilities|Casting|CastToABP_Enemy (Components|SkeletalMesh|GetAnimInstance (Variables|Character|GetMesh))))
  (Variables|/Game/AI/Enemy/Animations/ABP_Enemy.ABP_Enemy_C|SetState _asabp_enemy "NewEnumerator1"))

(fn GetState
  (bind _asabp_enemy (Utilities|Casting|CastToABP_Enemy (Components|SkeletalMesh|GetAnimInstance (Variables|Character|GetMesh))))
  (return (Variables|/Game/AI/Enemy/Animations/ABP_Enemy.ABP_Enemy_C|GetState _asabp_enemy)))