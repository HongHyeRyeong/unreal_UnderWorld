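; BP_CharacterEnemy is the AI enemy character that attacks survivors, installs traps, teleports and reacts to being hit.
; Actions set the ABP_Enemy state and flag BP_EnemyController as busy until EndAction.
; Attacks briefly enable a collision overlap, using a forward-vector dot product to tell survivors whether both face alike, and bind their counterattack to a delayed reaction.
; Hits during one particular state are ignored, and teleporting requires another, notifying the controller on success.
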(event OnComponentBeginOverlap(AttackCollision)
  (params (OverlappedComponent :type Primitive%20Component%20Object%20Reference) (OtherActor :type Actor%20Object%20Reference) (OtherComp :type Primitive%20Component%20Object%20Reference) (OtherBodyIndex :type Integer) (bFromSweep :type Boolean) (SweepResult :type Hit%20Result%20Structure%20%28by%20ref%29))
  (bind _asbp_survivor_character (Utilities|Casting|CastToBP_CharacterSurvivor OtherActor))
  (EventDispatchers|BindEventtoOnCounterAttacktoEnemy _asbp_survivor_character (delegate Custom|Event%20Counter%20Attack%20By%20Survivor))
  (Class|UnderWorldCharacter|AttackbyEnemy _asbp_survivor_character (>= (Math|Vector|DotProduct (Transformation|GetActorForwardVector _asbp_survivor_character) (Transformation|GetActorForwardVector self)) 0.0))
  (CallFunction|EventAttackEnd))

(event Custom|Event%20Attack%20End
  (Variables|/Script/Engine.PrimitiveComponent|SetbGenerateOverlapEvents (Variables|Default|GetAttackCollision) false))

(event Custom|Event%20End%20Action
  (bind _asbp_enemy_controller (Utilities|Casting|CastToBP_EnemyController (Pawn|GetController self)))
  (Default|EventSetAction _asbp_enemy_controller false))

(event Custom|Event%20Counter%20Attack%20By%20Survivor
  (Utilities|FlowControl|Delay 1.2)
  (CallFunction|EventPlayAction "NewEnumerator4"))

(event Custom|Event%20Play%20Action
  (params (state :type Enum_EnemyState%20Enum :default "NewEnumerator0"))
  (bind _asabp_enemy (Utilities|Casting|CastToABP_Enemy (Components|SkeletalMesh|GetAnimInstance (Variables|Character|GetMesh))))
  (Variables|/Game/AI/Enemy/Animations/ABP_Enemy.ABP_Enemy_C|SetState _asabp_enemy state)
  (bind _asbp_enemy_controller (Utilities|Casting|CastToBP_EnemyController (Pawn|GetController self)))
  (Default|EventSetAction _asbp_enemy_controller true))

(event Custom|Event%20Clear%20Game
  (CallFunction|EventPlayAction "NewEnumerator5"))

(event EventBeginPlay
  (CallFunction|EventAttackEnd))

(fn ConstructionScript)

(fn UpdateWalkSpeed
  (params (NewWalkSpeed :type Float%20%28double-precision%29))
  (Variables|/Script/Engine.CharacterMovementComponent|SetMaxWalkSpeed (Variables|Character|GetCharacterMovement) NewWalkSpeed))

(fn InstallTrap
  (Game|SpawnActorfromClass "/Game/Blueprints/BP_Trap.BP_Trap_C" (Transformation|GetWorldTransform (Variables|Default|GetTrapSpawn)) "Undefined" "MultiplyWithRoot" 0 0)
  (CallFunction|EventPlayAction "NewEnumerator2"))

(fn AttacktoSurvivor
  (Variables|/Script/Engine.PrimitiveComponent|SetbGenerateOverlapEvents (Variables|Default|GetAttackCollision) true)
  (CallFunction|EventPlayAction "NewEnumerator1"))

(fn AttackbySurvivor
  (bind _asabp_enemy (Utilities|Casting|CastToABP_Enemy (Components|SkeletalMesh|GetAnimInstance (Variables|Character|GetMesh))))
  (if (not (Utilities|Enum|Equal(Enum) (Variables|/Game/AI/Enemy/Animations/ABP_Enemy.ABP_Enemy_C|GetState _asabp_enemy) "NewEnumerator1"))
    (CallFunction|EventPlayAction "NewEnumerator4")))

(fn Teleport
  (params (transform :type Transform))
  (bind _asabp_enemy (Utilities|Casting|CastToABP_Enemy (Components|SkeletalMesh|GetAnimInstance (Variables|Character|GetMesh))))
  (if (Utilities|Enum|Equal(Enum) (Variables|/Game/AI/Enemy/Animations/ABP_Enemy.ABP_Enemy_C|GetState _asabp_enemy) "NewEnumerator0")
    (bind _returnvalue (Transformation|SetActorTransform transform false true))
    (if _returnvalue
      (bind _asbp_enemy_controller (Utilities|Casting|CastToBP_EnemyController (Pawn|GetController self)))
      (Default|EventTeleportEnd _asbp_enemy_controller)
      (return true)
      (else
        (return false)))
    (else
      (return false))))