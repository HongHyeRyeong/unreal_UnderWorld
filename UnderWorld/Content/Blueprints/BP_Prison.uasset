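; BP_Prison is a prison actor with a door that survivor characters can trigger while standing inside its capsule collision.
; On overlap it binds its DoorOpen event to the survivor's OnPrison dispatcher, so the door opens only when that dispatcher fires.
; DoorOpen plays a 2D sound and a timeline that rotates the door mesh.
; Any actor leaving the capsule reverses the timeline, and a departing survivor is unbound.
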(event OnComponentBeginOverlap(CapsuleCollision)
  (params (OverlappedComponent :type Primitive%20Component%20Object%20Reference) (OtherActor :type Actor%20Object%20Reference) (OtherComp :type Primitive%20Component%20Object%20Reference) (OtherBodyIndex :type Integer) (bFromSweep :type Boolean) (SweepResult :type Hit%20Result%20Structure%20%28by%20ref%29))
  (bind _asbp_character_survivor (Utilities|Casting|CastToBP_Character_Survivor OtherActor))
  (EventDispatchers|AssignOnPrison _asbp_character_survivor (delegate Custom|Event%20Door%20Open)))

(event OnComponentEndOverlap(CapsuleCollision)
  (params (OverlappedComponent :type Primitive%20Component%20Object%20Reference) (OtherActor :type Actor%20Object%20Reference) (OtherComp :type Primitive%20Component%20Object%20Reference) (OtherBodyIndex :type Integer))
  (CallFunction|EventDoorClose)
  (bind _asbp_character_survivor (Utilities|Casting|CastToBP_Character_Survivor OtherActor))
  (EventDispatchers|UnbindEventfromOnPrison _asbp_character_survivor (delegate Custom|Event%20Door%20Open)))

(event Custom|Event%20Door%20Open
  (Audio|PlaySound2D "/Game/Sound/S_Prison.S_Prison" 1.0 1.0 0.0 0 0)
  (bind _newtrack_0 (Timeline|Door%20Anim PlayFromStart)
    (:Update
      (Transformation|SetRelativeRotation (Variables|Default|GetSM_PrisonDoor) (Math|Rotator|Lerp(Rotator) "0, 0, 0" "0.000000,60.000000,0.000000" _newtrack_0 true) false false))))

(event Custom|Event%20Door%20Close
  (bind _newtrack_0 (Timeline|Door%20Anim Reverse)
    (:Update
      (Transformation|SetRelativeRotation (Variables|Default|GetSM_PrisonDoor) (Math|Rotator|Lerp(Rotator) "0, 0, 0" "0.000000,60.000000,0.000000" _newtrack_0 true) false false))))

(fn ConstructionScript)