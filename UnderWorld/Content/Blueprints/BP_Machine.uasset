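; BP_Machine is an objective machine where a survivor installs gadgets to end the game.
; The first survivor overlap binds install input and enables Tick, which advances progress by InstallSpeed and spins the wheel while overlap, input, gadget and count checks pass.
; Each full bar consumes a gadget; reaching the maximum swaps sparks for a completion light and calls GameMode's EventEndGame.
; Uncalled-here helpers spawn or teleport enemies to reachable points around EnemyPoint.
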(event Custom|Event%20Input%20Machine%20Install
  (params (active :type Boolean))
  ;[1 1 1] Init
  (Variables|Default|SetIsInput active))

(event EventTick
  (params (DeltaSeconds :type Float%20%28single-precision%29))
  (bind _install (CallFunction|CanInstall))
  (if _install
    ;[1 1 1] Begin Install
    (Utilities|FlowControl|Sequence
      (:then_0
        (if (not (Variables|Default|GetIsInstall))
          (Variables|Default|SetIsInstall true)
          (Class|UnderWorldCharacter|SetEState (Variables|Default|GetCharacter) "E_MachineInstall")))
      (:then_1
        (Variables|Default|SetInstall (+ (Variables|/Script/UnderWorld.UnderWorldCharacter|GetinstallSpeed (Variables|Default|GetCharacter)) (Variables|Default|GetInstall)))
        (CallFunction|PlayMachineWheel))
      (:then_2
        (if (>= (Variables|Default|GetInstall) 1e+02)
          (Class|UnderWorldCharacter|ItemRemove (Variables|Default|GetCharacter) "E_Gadget")
          (Variables|Default|SetInstall 0.0)
          (Variables|Default|SetCompleteCount (+ (Variables|Default|GetCompleteCount) 1)))))
    (else
      ;[1 1 1] End Install
      (if (Variables|Default|GetIsInstall)
        (Utilities|FlowControl|Sequence
          (:then_0
            (Variables|Default|SetIsInstall false)
            (Class|UnderWorldCharacter|SetEState (Variables|Default|GetCharacter) "E_Land"))
          (:then_1
            (if (>= (Variables|Default|GetCompleteCount) (Variables|Default|GetCompleteCountMax))
              (Rendering|SetVisibility (Variables|Default|GetCompleteLight) true false)
              (Rendering|SetVisibility (Variables|Default|GetP_Machine_Sparks) false false)
              (bind _asbp_game_mode (Utilities|Casting|CastToBP_GameMode (Game|GetGameMode)))
              (Default|EventEndGame _asbp_game_mode))))))))

(event Collision|EventActorBeginOverlap
  (params (OtherActor :type Actor%20Object%20Reference))
  (Variables|Default|SetIsOverlap true)
  ;[1 1 1] Init
  (if (not (Utilities|IsValid (Variables|Default|GetCharacter)))
    (bind _asbp_character_survivor (Utilities|Casting|CastToBP_Character_Survivor OtherActor))
    (bind _output_get (Variables|Default|SetCharacter _asbp_character_survivor))
    (EventDispatchers|BindEventtoOnInputMachineInstall _output_get (delegate Custom|Event%20Input%20Machine%20Install))
    (Actor|Tick|SetActorTickEnabled true)))

(event Collision|EventActorEndOverlap
  (params (OtherActor :type Actor%20Object%20Reference))
  (Variables|Default|SetIsOverlap false))

(fn ConstructionScript)

(fn PlayMachineWheel
  (Transformation|AddLocalRotation (Variables|Default|GetRoot%20MachineWheel) "0.000000,0.000000,2.000000" false false))

(fn CanInstall
  (return (Math|Boolean|ANDBoolean (Variables|Default|GetIsOverlap) (Variables|Default|GetIsInput) (Class|UnderWorldCharacter|IsHaveGadget (Variables|Default|GetCharacter)) (< (Variables|Default|GetCompleteCount) (Variables|Default|GetCompleteCountMax)))))

(fn SpawnEnemy
  (params (Radius :type Float%20%28double-precision%29))
  (bind _transform (CallFunction|GetRandomTransform Radius))
  (bind _returnvalue (Game|SpawnActorfromClass "/Game/AI/BP_Character_Enemy.BP_Character_Enemy_C" _transform "AdjustIfPossibleButAlwaysSpawn" "MultiplyWithRoot" 0 0))
  (return _returnvalue))

(fn TeleportEnemy
  (params (Radius :type Float%20%28double-precision%29))
  (bind _transform (CallFunction|GetRandomTransform Radius))
  (bind _returnvalue (Actor|GetActorOfClass "/Game/AI/BP_Character_Enemy.BP_Character_Enemy_C"))
  (bind _success (Default|Teleport _returnvalue _transform))
  (return _success))

(fn GetRandomTransform
  (params (Radius :type Float%20%28double-precision%29))
  (bind _output_get (LocalVariables|SetRandom%20Location (.RandomLocation (AI|Navigation|GetRandomReachablePointinRadius (Transformation|GetWorldLocation (Variables|Default|GetEnemy%20Point)) Radius 0 0))))
  (return (Math|Transform|MakeTransform _output_get (Math|Rotator|FindLookatRotation _output_get (Transformation|GetWorldLocation (Variables|Default|GetEnemy%20Point))))))