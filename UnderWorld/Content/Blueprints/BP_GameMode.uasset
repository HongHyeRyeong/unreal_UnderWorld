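; Game mode that triggers enemy spawning and provides item placement for the level.
; On BeginPlay it gathers all BP_Machine actors and, after a short delay, tells a random one to spawn an enemy.
; SpawnItems, not called within this Blueprint, places leveled hats and bags plus keys on "Item"-tagged spawn points, then gadgets on "Gadget"-tagged ones.
; Each random pick removes that point from the pool, preventing reuse.
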(event EventBeginPlay
  (bind _outactors (Actor|GetAllActorsOfClass "/Game/Blueprints/BP_Machine.BP_Machine_C"))
  (Variables|Default|SetMachines _outactors)
  (Utilities|FlowControl|Delay 5.0)
  (Default|SpawnEnemy (.OutItem (Utilities|Array|Random (Variables|Default|GetMachines)))))

(fn ConstructionScript)

(fn SpawnItems
  (params (MaxHatLevel :type Integer) (MaxBagLevel :type Integer))
  (Utilities|FlowControl|Sequence
    (:then_0
      (bind _outactors (Actor|GetAllActorsOfClasswithTag "/Game/Blueprints/BP_SpawnPoint.BP_SpawnPoint_C" "Item"))
      (Variables|Default|SetItem%20Spawn%20Points _outactors)
      (Utilities|FlowControl|Sequence
        (:then_0
          (for _index (range 1 MaxHatLevel)
            (bind _spawn_transform (CallFunction|GetTransformonItemSpawnPoints))
            (bind _returnvalue (Game|SpawnActorfromClass "/Game/Blueprints/BP_Item_Hat.BP_Item_Hat_C" _spawn_transform "AdjustIfPossibleButAlwaysSpawn" "MultiplyWithRoot" 0 0))
            (Default|SetLevel _returnvalue _index)))
        (:then_1
          (for _index_2 (range 1 MaxBagLevel)
            (bind _spawn_transform_2 (CallFunction|GetTransformonItemSpawnPoints))
            (bind _returnvalue_2 (Game|SpawnActorfromClass "/Game/Blueprints/BP_Item_Bag.BP_Item_Bag_C" _spawn_transform_2 "AdjustIfPossibleButAlwaysSpawn" "MultiplyWithRoot" 0 0))
            (Default|SetLevel _returnvalue_2 _index_2)))
        (:then_2
          (for _index_3 (range 1 3)
            (bind _spawn_transform_3 (CallFunction|GetTransformonItemSpawnPoints))
            (Game|SpawnActorfromClass "/Game/Blueprints/BP_Item_Key.BP_Item_Key_C" _spawn_transform_3 "AdjustIfPossibleButAlwaysSpawn" "MultiplyWithRoot" 0 0)))))
    (:then_1
      (bind _outactors_2 (Actor|GetAllActorsOfClasswithTag "/Game/Blueprints/BP_SpawnPoint.BP_SpawnPoint_C" "Gadget"))
      (Variables|Default|SetItem%20Spawn%20Points _outactors_2)
      (for _index_4 (range 1 10)
        (bind _spawn_transform_4 (CallFunction|GetTransformonItemSpawnPoints))
        (Game|SpawnActorfromClass "/Game/Blueprints/BP_Item_Gadget.BP_Item_Gadget_C" _spawn_transform_4 "AdjustIfPossibleButAlwaysSpawn" "MultiplyWithRoot" 0 0)))))

(fn GetTransformonItemSpawnPoints
  (LocalVariables|SetSpawn%20Point (.OutItem (Utilities|Array|Random (Variables|Default|GetItem%20Spawn%20Points))))
  (LocalVariables|SetTransform (Math|Transform|MakeTransform (Transformation|GetActorLocation (LocalVariables|GetSpawn%20Point))))
  (Utilities|Array|RemoveItem (Variables|Default|GetItem%20Spawn%20Points) (LocalVariables|GetSpawn%20Point))
  (return (LocalVariables|GetTransform)))