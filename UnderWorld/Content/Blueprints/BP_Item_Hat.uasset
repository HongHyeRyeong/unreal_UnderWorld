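; BP_Item_Hat is a hat item Blueprint that shows its item level and highlight state on the SMHat mesh.
; SetLevel stores the level in ItemLevel and switches the mesh's first material slot among three survivor item materials, one per level.
; SetOutline toggles an outline by applying or clearing an overlay material on the same mesh, leaving the level material in place.
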(event Custom|Set%20Level
  (params (level :type Integer))
  (bind _sm_hat (Variables|Default|GetSM_Hat))
  (bind _output_get (Variables|Default|SetitemLevel level))
  (switch int _output_get
    (:1
      (Rendering|Material|SetMaterial _sm_hat 0 "/Game/Item/Materials/M_Item_Survivor_Level1.M_Item_Survivor_Level1"))
    (:2
      (Rendering|Material|SetMaterial _sm_hat 0 "/Game/Item/Materials/M_Item_Survivor_Level2.M_Item_Survivor_Level2"))
    (:3
      (Rendering|Material|SetMaterial _sm_hat 0 "/Game/Item/Materials/M_Item_Survivor_Level3.M_Item_Survivor_Level3"))))

(event EventSetOutline
  (params (active :type Boolean))
  (bind _sm_hat (Variables|Default|GetSM_Hat))
  (if active
    (Rendering|Material|SetOverlayMaterial _sm_hat "/Game/Item/Materials/M_Outline.M_Outline" :!class /Script/Engine.MeshComponent)
    (else
      (Rendering|Material|SetOverlayMaterial _sm_hat 0 :!class /Script/Engine.MeshComponent))))

(fn ConstructionScript)