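; BP_Door is a button-operated door that keeps an enemy out, with a warning light driven by layered trigger volumes.
; Holding the button briefly closes it temporarily; the door at the first "Door"-tagged spawn point also has BP_GameMode teleport the enemy.
; Trigger overlaps step the light from green through orange and red to blinking.
; Entering the Dead trigger while open shuts and locks every door and notifies the enemy's AI controller.
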(event OnComponentBeginOverlap(Collision)
  (params (OverlappedComponent :type Primitive%20Component%20Object%20Reference) (OtherActor :type Actor%20Object%20Reference) (OtherComp :type Primitive%20Component%20Object%20Reference) (OtherBodyIndex :type Integer) (bFromSweep :type Boolean) (SweepResult :type Hit%20Result%20Structure%20%28by%20ref%29))
  ;[1 1 1] Door Button
  (CallFunction|EventButtonDown)
  (bind _returnvalue (Utilities|Time|SetTimerbyEvent (delegate Custom|Event%20Door%20CloseAndOpen) 0.5))
  (Variables|Default|SetTimer%20Door%20Button _returnvalue))

(event OnComponentEndOverlap(Collision)
  (params (OverlappedComponent :type Primitive%20Component%20Object%20Reference) (OtherActor :type Actor%20Object%20Reference) (OtherComp :type Primitive%20Component%20Object%20Reference) (OtherBodyIndex :type Integer))
  ;[1 1 1] Door Button
  (CallFunction|EventButtonUp)
  (Utilities|Time|ClearandInvalidateTimerbyHandle (Variables|Default|GetTimer%20Door%20Button)))

(event OnComponentBeginOverlap(Orange)
  (params (OverlappedComponent :type Primitive%20Component%20Object%20Reference) (OtherActor :type Actor%20Object%20Reference) (OtherComp :type Primitive%20Component%20Object%20Reference) (OtherBodyIndex :type Integer) (bFromSweep :type Boolean) (SweepResult :type Hit%20Result%20Structure%20%28by%20ref%29))
  ;[1 1 1] Door Light
  (CallFunction|EventSetState 1))

(event OnComponentEndOverlap(Orange)
  (params (OverlappedComponent :type Primitive%20Component%20Object%20Reference) (OtherActor :type Actor%20Object%20Reference) (OtherComp :type Primitive%20Component%20Object%20Reference) (OtherBodyIndex :type Integer))
  ;[1 1 1] Door Light
  (CallFunction|EventSetState))

(event OnComponentBeginOverlap(Red)
  (params (OverlappedComponent :type Primitive%20Component%20Object%20Reference) (OtherActor :type Actor%20Object%20Reference) (OtherComp :type Primitive%20Component%20Object%20Reference) (OtherBodyIndex :type Integer) (bFromSweep :type Boolean) (SweepResult :type Hit%20Result%20Structure%20%28by%20ref%29))
  ;[1 1 1] Door Light
  (CallFunction|EventSetState 2))

(event OnComponentEndOverlap(Red)
  (params (OverlappedComponent :type Primitive%20Component%20Object%20Reference) (OtherActor :type Actor%20Object%20Reference) (OtherComp :type Primitive%20Component%20Object%20Reference) (OtherBodyIndex :type Integer))
  ;[1 1 1] Door Light
  (CallFunction|EventSetState 1))

(event OnComponentBeginOverlap(DarkRed)
  (params (OverlappedComponent :type Primitive%20Component%20Object%20Reference) (OtherActor :type Actor%20Object%20Reference) (OtherComp :type Primitive%20Component%20Object%20Reference) (OtherBodyIndex :type Integer) (bFromSweep :type Boolean) (SweepResult :type Hit%20Result%20Structure%20%28by%20ref%29))
  ;[1 1 1] Door Light
  (CallFunction|EventSetState 3))

(event OnComponentEndOverlap(DarkRed)
  (params (OverlappedComponent :type Primitive%20Component%20Object%20Reference) (OtherActor :type Actor%20Object%20Reference) (OtherComp :type Primitive%20Component%20Object%20Reference) (OtherBodyIndex :type Integer))
  ;[1 1 1] Door Light
  (CallFunction|EventSetState 2))

(event OnComponentBeginOverlap(Dead)
  (params (OverlappedComponent :type Primitive%20Component%20Object%20Reference) (OtherActor :type Actor%20Object%20Reference) (OtherComp :type Primitive%20Component%20Object%20Reference) (OtherBodyIndex :type Integer) (bFromSweep :type Boolean) (SweepResult :type Hit%20Result%20Structure%20%28by%20ref%29))
  ;[1 1 1] Door Light
  (if (Variables|Default|GetDoor%20Open)
    (Utilities|FlowControl|Sequence
      (:then_0
        (for _array_element (Variables|Default|GetDorrs)
          (CallFunction|EventRestartGame _array_element)))
      (:then_1
        (bind _asbp_character_enemy (Utilities|Casting|CastToBP_CharacterEnemy OtherActor))
        (bind _asbp_enemy_controller (Utilities|Casting|CastToBP_EnemyController (AI|GetAIController _asbp_character_enemy)))
        (Default|EventDoorInside _asbp_enemy_controller)))))

(event Custom|Event%20Button%20Down
  ;[1 1 1] Door Button
  (bind _newtrack_0 (Timeline|Button%20Up/Down PlayFromStart)
    (:Update
      (Transformation|SetRelativeLocation (Variables|Default|GetButtons) (Math|Vector|Lerp(Vector) "0, 0, 0" "0.000000,0.000000,-4.000000" _newtrack_0) false false))))

(event Custom|Event%20Button%20Up
  ;[1 1 1] Door Button
  (bind _newtrack_0 (Timeline|Button%20Up/Down Reverse)
    (:Update
      (Transformation|SetRelativeLocation (Variables|Default|GetButtons) (Math|Vector|Lerp(Vector) "0, 0, 0" "0.000000,0.000000,-4.000000" _newtrack_0) false false))))

(event Custom|Event%20Set%20State
  (params (state :type Integer))
  (bind _light (Variables|Default|GetLight))
  (bind _light_2 (Variables|Default|GetLight))
  ;[1 1 1] Set Light State
  (if (not (Variables|Default|GetRestart%20Game))
    (Utilities|FlowControl|Sequence
      (:then_0
        (bind _light_3 (Timeline|Light%20Blink Stop)
          (:Update
            (if (>= _light_3 1.0)
              (Rendering|Material|SetMaterial _light_2 0 "/Game/MapObject/Materials/M_Emissive_Red.M_Emissive_Red")
              (else
                (Rendering|Material|SetMaterial _light_2 0 "/Game/MapObject/Materials/M_Emissive_DarkRed.M_Emissive_DarkRed"))))))
      (:then_1
        (switch int state
          (:0
            (Rendering|Material|SetMaterial _light 0 "/Game/MapObject/Materials/M_Emissive_Green.M_Emissive_Green"))
          (:1
            (Rendering|Material|SetMaterial _light 0 "/Game/MapObject/Materials/M_Emissive_Orange.M_Emissive_Orange"))
          (:2
            (Rendering|Material|SetMaterial _light 0 "/Game/MapObject/Materials/M_Emissive_Red.M_Emissive_Red"))
          (:3
            (Timeline|Light%20Blink PlayFromStart)))))))

(event Custom|Event%20Door%20Open
  ;[1 1 1] Door
  (if (not (Variables|Default|GetRestart%20Game))
    (Variables|Default|SetDoor%20Open true)
    (Audio|PlaySound2D "/Game/Sound/S_DoorOpen.S_DoorOpen" 1.0 3.0 0.0 0 0)
    (bind _newtrack_0 (Timeline|Door%20Open/Close PlayFromStart)
      (:Update
        (Transformation|SetRelativeLocation (Variables|Default|GetDoors) (Math|Vector|Lerp(Vector) "0, 0, 0" "0.000000,370.000000,0.000000" _newtrack_0) false false)))))

(event Custom|Event%20Door%20Close
  (params (Called%20Restart%20Game :type Boolean))
  ;[1 1 1] Door
  (if (not (Variables|Default|GetRestart%20Game))
    (Variables|Default|SetDoor%20Open false)
    (Audio|PlaySound2D "/Game/Sound/S_DoorClose.S_DoorClose" 0.8 1.0 0.0 0 0)
    (if Called%20Restart%20Game
      (bind _newtrack_0 (Timeline|Door%20Open/Close ReverseFromEnd)
        (:Update
          (Transformation|SetRelativeLocation (Variables|Default|GetDoors) (Math|Vector|Lerp(Vector) "0, 0, 0" "0.000000,370.000000,0.000000" _newtrack_0) false false)))
      (else
        (Utilities|FlowControl|Sequence
          (:then_0
            (Timeline|Door%20Open/Close ReverseFromEnd))
          (:then_1
            (if (Utilities|Operators|EqualEqual (Transformation|GetActorLocation (Variables|Default|GetDoor%20Point)) (Transformation|GetActorLocation) 0.0)
              (Utilities|FlowControl|Delay 2.0)
              (bind _asbp_game_mode (Utilities|Casting|CastToBP_GameMode (Game|GetGameMode)))
              (Default|TeleportEnemy _asbp_game_mode)
              (CallFunction|EventSetState))))))))

(event Custom|Event%20Start%20Game
  (CallFunction|EventSetState)
  (CallFunction|EventDoorOpen))

(event Custom|Event%20Restart%20Game
  (CallFunction|EventSetState 3)
  (CallFunction|EventDoorClose true)
  (Variables|Default|SetRestart%20Game true))

(event Custom|Event%20Door%20CloseAndOpen
  ;[1 1 1] Door
  (CallFunction|EventDoorClose false)
  (Utilities|Time|SetTimerbyEvent (delegate Custom|Event%20Door%20Open) 3.0))

(event EventBeginPlay
  (CallFunction|EventStartGame)
  (bind _outactors (Actor|GetAllActorsOfClasswithTag "/Game/Blueprints/BP_SpawnPoint.BP_SpawnPoint_C" "Door"))
  (Variables|Default|SetDoor%20Point (Utilities|Array|Get(acopy) _outactors))
  (bind _outactors_2 (Actor|GetAllActorsOfClass "BP_Door_C"))
  (Variables|Default|SetDorrs _outactors_2))

(fn ConstructionScript)