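; Survivor character Blueprint that handles worn items, machine installation and melee attacks against enemies.
; Equipping a hat or bag toggles its mesh and swaps in a material by item level.
; Machine installation is forwarded to the survivor animation Blueprint, and completion removes the gadget item.
; State changes enable attack collision overlaps only while attacking, and overlapped enemies take survivor damage unless in one excluded state.
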(event OnComponentBeginOverlap(AttackCollision)
  (params (OverlappedComponent :type Primitive%20Component%20Object%20Reference) (OtherActor :type Actor%20Object%20Reference) (OtherComp :type Primitive%20Component%20Object%20Reference) (OtherBodyIndex :type Integer) (bFromSweep :type Boolean) (SweepResult :type Hit%20Result%20Structure%20%28by%20ref%29))
  (bind _asbp_character_enemy (Utilities|Casting|CastToBP_Character_Enemy OtherActor))
  (bind _state (Default|GetState _asbp_character_enemy))
  (if (not (Utilities|Enum|Equal(Enum) _state "NewEnumerator1"))
    (Default|EventDamagebySurvivor _asbp_character_enemy)))

(event Custom|Event%20Attack%20End
  (Variables|/Script/Engine.PrimitiveComponent|SetbGenerateOverlapEvents (Variables|Default|GetAttackCollision) false))

(event Custom|Event%20Machine%20Install
  (params (Install :type Boolean))
  (bind _asabp_survivor (Utilities|Casting|CastToABP_Survivor (Components|SkeletalMesh|GetAnimInstance (Variables|Character|GetMesh))))
  (Default|EventMachineInstall _asabp_survivor Install))

(event Custom|Event%20Machine%20Complete
  (Class|UnderWorldCharacter|ItemRemove "E_Gadget"))

(event Custom|Event%20Set%20State
  (params (state :type EState%20Enum :default "E_Land"))
  (if (Utilities|Enum|Equal(Enum) state "E_Attack")
    (Variables|/Script/Engine.PrimitiveComponent|SetbGenerateOverlapEvents (Variables|Default|GetAttackCollision) true)
    (else
      (CallFunction|EventAttackEnd))))

(event EventBeginPlay
  (EventDispatchers|BindEventtoOnChangeState (delegate Custom|Event%20Set%20State))
  (CallFunction|EventAttackEnd))

(event EventItemPuton
  (params (type :type EItemType%20Enum :default "E_Hat") (level :type Integer))
  (bind _sm_bag (Variables|Default|GetSM_Bag))
  (bind _sm_hat (Variables|Default|GetSM_Hat))
  (switch Utilities|FlowControl|Switch|SwitchonEItemType type
    (:E_Hat
      (Rendering|SetVisibility _sm_hat (> level 0) false)
      (switch int level
        (:Default
          (Rendering|Material|SetMaterial _sm_hat 0 "/Game/Item/Materials/M_Item_Survivor_Level1.M_Item_Survivor_Level1" :!label _label))
        (:1
          (goto _label))
        (:2
          (Rendering|Material|SetMaterial _sm_hat 0 "/Game/Item/Materials/M_Item_Survivor_Level2.M_Item_Survivor_Level2"))
        (:3
          (Rendering|Material|SetMaterial _sm_hat 0 "/Game/Item/Materials/M_Item_Survivor_Level3.M_Item_Survivor_Level3"))))
    (:E_Bag
      (Rendering|SetVisibility _sm_bag (> level 0) false)
      (switch int level
        (:1
          (Rendering|Material|SetMaterial _sm_bag 0 "/Game/Item/Materials/M_Item_Survivor_Level1.M_Item_Survivor_Level1"))
        (:2
          (Rendering|Material|SetMaterial _sm_bag 0 "/Game/Item/Materials/M_Item_Survivor_Level2.M_Item_Survivor_Level2"))))))

(fn ConstructionScript)